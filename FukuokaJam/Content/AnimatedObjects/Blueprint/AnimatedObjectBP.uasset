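; Animated skeletal mesh actor whose animation playback is scrubbed by the player pawn's position along the world X axis.
; The construction script applies the configurable mesh and AnimBP class.
; Each tick, it converts the X offset to the player into a time centered on half the animation length, wrapped when looping or clamped otherwise.
; That time is passed to the anim instance through AnimationTimeInterface.
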(event EventBeginPlay)

(event Collision|EventActorBeginOverlap
  (params (OtherActor :type Actor%20Object%20Reference)))

(event EventTick
  (params (DeltaSeconds :type Float%20%28single-precision%29))
  ;[0.15 0.15 0.15 0.5] Update AnimBP Time Value
  (bind _asanimation_time_interface (Utilities|Casting|CastToAnimationTimeInterface (Components|SkeletalMesh|GetAnimInstance (Variables|Default|GetSkeletalMesh))))
  (Default|SetTime _asanimation_time_interface (CallFunction|CalculateAnimationTime (- (.x (Transformation|GetActorLocation)) (.x (Transformation|GetActorLocation (Game|Player|GetPlayerPawn 0)))) (Variables|Default|GetLooping))))

(fn ConstructionScript
  (Components|SkeletalMesh|SetSkeletalMeshAsset (Variables|Default|GetSkeletalMesh) (Variables|Default|GetSkeletalMeshAsset))
  (Components|SkeletalMesh|SetAnimInstanceClass (Variables|Default|GetSkeletalMesh) (Variables|Default|GetAnimationAsset)))

(fn CalculateAnimationTime
  (params (Distance :type Float%20%28double-precision%29) (Looping :type Boolean))
  (bind _animationdistance (Variables|Default|GetAnimationDistance))
  (bind _animationlength (Variables|Default|GetAnimationLength))
  (bind _returnvalue (/ _animationlength -2.0))
  (bind _returnvalue_2 (* Distance _animationdistance))
  (bind _returnvalue_3 (Utilities|Operators|Subtract _returnvalue_2 _returnvalue))
  (if Looping
    (return (Math|Float|%(Float) (+ _returnvalue_3 (* (Variables|Default|GetAnimationLength) 1e+01)) (Variables|Default|GetAnimationLength)))
    (else
      (return (Math|Float|Clamp(Float) _returnvalue_3 0.0 (Variables|Default|GetAnimationLength))))))