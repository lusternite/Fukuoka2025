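; Conveyor belt actor that carries the first-person player along one of four directions while they overlap its box collision.
; The construction script gives both belt meshes a shared dynamic material, colored by ConveyorDirection.
; Each tick, the player's absolute world-X velocity, normalized and clamped, drives both the material's smoothed Speed parameter and a swept location offset along the belt.
; The belt's push therefore scales with player movement on X.
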(event OnComponentBeginOverlap(BoxCollision)
  (params (OverlappedComponent :type Primitive%20Component%20Object%20Reference) (OtherActor :type Actor%20Object%20Reference) (OtherComp :type Primitive%20Component%20Object%20Reference) (OtherBodyIndex :type Integer) (bFromSweep :type Boolean) (SweepResult :type Hit%20Result%20Structure%20%28by%20ref%29))
  (Utilities|Casting|CastToBP_FirstPersonCharacter OtherActor)
  (Variables|Default|SetOnConveyor true))

(event OnComponentEndOverlap(BoxCollision)
  (params (OverlappedComponent :type Primitive%20Component%20Object%20Reference) (OtherActor :type Actor%20Object%20Reference) (OtherComp :type Primitive%20Component%20Object%20Reference) (OtherBodyIndex :type Integer))
  (Utilities|Casting|CastToBP_FirstPersonCharacter OtherActor)
  (Variables|Default|SetOnConveyor false))

(event EventBeginPlay
  (bind _asbp_first_person_character (Utilities|Casting|CastToBP_FirstPersonCharacter (Game|Player|GetPlayerPawn 0)))
  (Variables|Default|SetPlayerCharacter _asbp_first_person_character))

(event Collision|EventActorBeginOverlap
  (params (OtherActor :type Actor%20Object%20Reference)))

(event EventTick
  (params (DeltaSeconds :type Float%20%28single-precision%29))
  (bind _conveyormat (Variables|Default|GetConveyorMat))
  (bind _playercharacter (Variables|Default|GetPlayerCharacter))
  (bind _playercharacter_2 (Variables|Default|GetPlayerCharacter))
  (bind _returnvalue (Transformation|GetVelocity _playercharacter))
  (bind _returnvalue_2 (/ (.x _returnvalue) 6e+02))
  (bind _returnvalue_3 (Math|Float|Absolute(Float) _returnvalue_2))
  (bind _returnvalue_4 (Math|Float|Clamp(Float) _returnvalue_3))
  (bind _returnvalue_5 (Rendering|Material|GetScalarParameterValue _conveyormat "Speed" :!class /Script/Engine.MaterialInstanceDynamic))
  (Rendering|Material|SetScalarParameterValue _conveyormat "Speed" (Math|Float|Lerp _returnvalue_5 _returnvalue_4 0.7) :!class /Script/Engine.MaterialInstanceDynamic)
  (if (Variables|Default|GetOnConveyor)
    (Transformation|SetActorLocation _playercharacter_2 (+ (Transformation|GetActorLocation _playercharacter_2) (* (* (* (Utilities|GetConveyorDirection) DeltaSeconds) 6e+02) _returnvalue_4)) true false)
    (else
      (Variables|Default|SetLastPlayerXLocation (.x (Transformation|GetActorLocation (Variables|Default|GetPlayerCharacter)))))))

(fn ConstructionScript
  (bind _returnvalue (Rendering|Material|CreateDynamicMaterialInstance "/Game/AnimatedObjects/Assets/Conveyor/Materials/ConveyorMat.ConveyorMat" "None" "None" :!class /Script/Engine.KismetMaterialLibrary))
  (Variables|Default|SetConveyorMat _returnvalue)
  (Rendering|Material|SetMaterial (Variables|Default|GetConveyor1) 0 (Variables|Default|GetConveyorMat))
  (Rendering|Material|SetMaterial (Variables|Default|GetConveyor2) 0 (Variables|Default|GetConveyorMat))
  (Rendering|Material|SetVectorParameterValue (Variables|Default|GetConveyorMat) "Color" (Utilities|Select :Index (Variables|Default|GetConveyorDirection) :Option%200 "(R=0.000000,G=1.000000,B=0.045295,A=1.000000)" :Option%201 "(R=1.000000,G=0.066702,B=0.000000,A=1.000000)" :Option%202 "(R=0.990708,G=1.000000,B=0.000000,A=1.000000)" :Option%203 "(R=1.000000,G=0.938762,B=0.000000,A=1.000000)") :!class /Script/Engine.MaterialInstanceDynamic))