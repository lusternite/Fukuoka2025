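; Background music controller that crossfades three music layers (forward, stopped and backward) to match the player's movement along the world X axis.
; Every Tick it reads the sign of the player character's X velocity to pick the active layer.
; FInterpTo on each audio component's volume multiplier raises that layer and fades out the other two at a shared InterpSpeed.
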(event EventBeginPlay)

(event Collision|EventActorBeginOverlap
  (params (OtherActor :type Actor%20Object%20Reference)))

(event EventTick
  (params (DeltaSeconds :type Float%20%28single-precision%29))
  (bind _time_relative_stopped (Variables|Default|GetTime_Relative_Stopped))
  (bind _time_relative_backward (Variables|Default|GetTime_Relative_Backward))
  (bind _time_relative_foward (Variables|Default|GetTime_Relative_Foward))
  (bind _time_relative_stopped_2 (Variables|Default|GetTime_Relative_Stopped))
  (bind _time_relative_backward_2 (Variables|Default|GetTime_Relative_Backward))
  (bind _time_relative_foward_2 (Variables|Default|GetTime_Relative_Foward))
  (bind _time_relative_stopped_3 (Variables|Default|GetTime_Relative_Stopped))
  (bind _time_relative_backward_3 (Variables|Default|GetTime_Relative_Backward))
  (bind _time_relative_foward_3 (Variables|Default|GetTime_Relative_Foward))
  (bind _output_get (Variables|Default|SetXVelocity (.X (Math|Vector|BreakVector (Transformation|GetVelocity (Game|GetPlayerCharacter 0))))))
  (if (> _output_get 0.0)
    (Audio|Components|Audio|SetVolumeMultiplier _time_relative_foward_3 (Math|Interpolation|FInterpTo (Variables|/Script/Engine.AudioComponent|GetVolumeMultiplier _time_relative_foward_3) 1.0 (Utilities|Time|GetWorldDeltaSeconds) (Variables|Default|GetInterpSpeed)) :!class /Script/Engine.AudioComponent)
    (Audio|Components|Audio|SetVolumeMultiplier _time_relative_stopped (Math|Interpolation|FInterpTo (Variables|/Script/Engine.AudioComponent|GetVolumeMultiplier _time_relative_stopped) 0.0 (Utilities|Time|GetWorldDeltaSeconds) (Variables|Default|GetInterpSpeed)) :!class /Script/Engine.AudioComponent)
    (Audio|Components|Audio|SetVolumeMultiplier _time_relative_backward (Math|Interpolation|FInterpTo (Variables|/Script/Engine.AudioComponent|GetVolumeMultiplier _time_relative_backward) 0.0 (Utilities|Time|GetWorldDeltaSeconds) (Variables|Default|GetInterpSpeed)) :!class /Script/Engine.AudioComponent)
    (elif (< _output_get 0.0)
      (Audio|Components|Audio|SetVolumeMultiplier _time_relative_foward (Math|Interpolation|FInterpTo (Variables|/Script/Engine.AudioComponent|GetVolumeMultiplier _time_relative_foward) 0.0 (Utilities|Time|GetWorldDeltaSeconds) (Variables|Default|GetInterpSpeed)) :!class /Script/Engine.AudioComponent)
      (Audio|Components|Audio|SetVolumeMultiplier _time_relative_stopped_2 (Math|Interpolation|FInterpTo (Variables|/Script/Engine.AudioComponent|GetVolumeMultiplier _time_relative_stopped_2) 0.0 (Utilities|Time|GetWorldDeltaSeconds) (Variables|Default|GetInterpSpeed)) :!class /Script/Engine.AudioComponent)
      (Audio|Components|Audio|SetVolumeMultiplier _time_relative_backward_2 (Math|Interpolation|FInterpTo (Variables|/Script/Engine.AudioComponent|GetVolumeMultiplier _time_relative_backward_2) 1.0 (Utilities|Time|GetWorldDeltaSeconds) (Variables|Default|GetInterpSpeed)) :!class /Script/Engine.AudioComponent)
      (else
        (Audio|Components|Audio|SetVolumeMultiplier _time_relative_foward_2 (Math|Interpolation|FInterpTo (Variables|/Script/Engine.AudioComponent|GetVolumeMultiplier _time_relative_foward_2) 0.0 (Utilities|Time|GetWorldDeltaSeconds) (Variables|Default|GetInterpSpeed)) :!class /Script/Engine.AudioComponent)
        (Audio|Components|Audio|SetVolumeMultiplier _time_relative_stopped_3 (Math|Interpolation|FInterpTo (Variables|/Script/Engine.AudioComponent|GetVolumeMultiplier _time_relative_stopped_3) 1.0 (Utilities|Time|GetWorldDeltaSeconds) (Variables|Default|GetInterpSpeed)) :!class /Script/Engine.AudioComponent)
        (Audio|Components|Audio|SetVolumeMultiplier _time_relative_backward_3 (Math|Interpolation|FInterpTo (Variables|/Script/Engine.AudioComponent|GetVolumeMultiplier _time_relative_backward_3) 0.0 (Utilities|Time|GetWorldDeltaSeconds) (Variables|Default|GetInterpSpeed)) :!class /Script/Engine.AudioComponent)))))

(fn ConstructionScript)